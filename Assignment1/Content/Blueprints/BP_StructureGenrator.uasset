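; BP_StructureGenrator is a block structure generator that, as wired, spawns only one static mesh component at BeginPlay, scaled by BlockGroesse.
; An unconnected nested loop would add three blocks per level across AnzahlEbenen levels, applying BlockMaterial and alternating rotation on even and odd levels.
; That loop never runs, its height-offset calculation feeds nothing, and the construction script is empty.
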(event EventBeginPlay
  (bind _returnvalue (AddComponent|AddStaticMeshComponent false))
  (Rendering|Material|SetMaterial _returnvalue 0 0)
  (Transformation|SetWorldScale3D _returnvalue (Variables|Default|GetBlockGroesse))
  (Transformation|SetRelativeLocationAndRotation _returnvalue "0, 0, 0" "0, 0, 0" false false))

(fn ConstructionScript)