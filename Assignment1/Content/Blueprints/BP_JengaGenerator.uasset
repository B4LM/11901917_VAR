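; Generator actor that builds a ring-shaped, polygonal Jenga tower from BP_JengaBlock actors on BeginPlay.
; RebuildTower, intended for reuse by other Blueprints, keeps the first block found as a size reference and destroys the rest.
; Nested loops spawn each level's blocks around StartLoc, using trigonometry for polygon radius and yaw.
; Alternate levels shift by half an angular step to stagger the blocks.
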(event EventBeginPlay
  (CallFunction|RebuildTower) ; Function to use in other blueprint for rebuilding the tower
)

(fn ConstructionScript)

(fn RebuildTower
  (bind _blocknumberperstage (Variables|Default|GetBlockNumberPerStage))
  (bind _returnvalue (/ 360 _blocknumberperstage))
  (bind _outactors (Actor|GetAllActorsOfClass "/Game/Blueprints/BP_JengaBlock.BP_JengaBlock_C"))
  ;[0.15 0.15 0.15 0.5] get Jenga-Block Dimensions
  (bind _asbp_jenga_block (Utilities|Casting|CastToBP_JengaBlock (Utilities|Array|Get(acopy) _outactors)))
  (Utilities|Array|RemoveIndex _outactors) ; Leave first Block in Game as reference
  ;[0.15 0.15 0.15 0.5] check if Tower already exists
  (if (> (Utilities|Array|Length _outactors) 0)
    ;[0.15 0.15 0.15 0.5] Delete Actors for Rebuilding
    (for _array_element _outactors
      (Actor|DestroyActor _array_element)))
  (Development|PrintText "BuildingTower")
  ;[0.15 0.15 0.15 0.5] Building Loops
  (for _index (range 0 (- (Variables|Default|GetTowerHight) 1)) ; Tower Hight
    (for _index_2 (range 0 (- _blocknumberperstage 1)) ; Tower Level
      ;[0.15 0.15 0.15 0.5] Spawn Jenga-Block
      (Game|SpawnActorfromClass "/Game/Blueprints/BP_JengaBlock.BP_JengaBlock_C" (Math|Transform|MakeTransform (+ (+ (Math|Vector|RotateVector (select (== (Math|Integer|%(Integer) _index 2) 0) (Math|Vector|MakeVector (Math|Float|Sqrt (- (Math|Float|Square (/ (* (.Y (Math|Vector|BreakVector (Variables|/Game/Blueprints/BP_JengaBlock.BP_JengaBlock_C|GetJBlockDimensions _asbp_jenga_block))) 1e+02) (* 2.0 (Math|Trig|Sin(Degrees) (Math|Conversions|ToFloat(Integer) (/ _returnvalue 2)))))) (Math|Float|Square (/ (* (.Y (Math|Vector|BreakVector (Variables|/Game/Blueprints/BP_JengaBlock.BP_JengaBlock_C|GetJBlockDimensions _asbp_jenga_block))) 1e+02) 2.0)))) (* (/ (* (.Y (Math|Vector|BreakVector (Variables|/Game/Blueprints/BP_JengaBlock.BP_JengaBlock_C|GetJBlockDimensions _asbp_jenga_block))) 1e+02) 2.0) -1.0) 0.0) (Math|Vector|MakeVector (/ (* (.Y (Math|Vector|BreakVector (Variables|/Game/Blueprints/BP_JengaBlock.BP_JengaBlock_C|GetJBlockDimensions _asbp_jenga_block))) 1e+02) (* 2.0 (Math|Trig|Sin(Degrees) (Math|Conversions|ToFloat(Integer) (/ _returnvalue 2))))) 0.0 0.0)) (Math|Rotator|MakeRotator 0.0 0.0 (* (Math|Conversions|ToFloat(Integer) (* _index_2 _returnvalue)) -1.0))) (Variables|Default|GetStartLoc)) (Math|Vector|MakeVector 0.0 0.0 (+ (* (* (.Z (Math|Vector|BreakVector (Variables|/Game/Blueprints/BP_JengaBlock.BP_JengaBlock_C|GetJBlockDimensions _asbp_jenga_block))) 1e+02) _index) 0.005))) (Math|Rotator|MakeRotator 0.0 0.0 (* (Math|Conversions|ToFloat(Integer) (select (== (Math|Integer|%(Integer) _index 2) 0) (* _index_2 _returnvalue) (- (* _index_2 _returnvalue) (/ _returnvalue 2)))) -1.0))) "Undefined" "MultiplyWithRoot" 0 0))))