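; BP_BoxAssembler builds a cubic box at runtime from six BP_BoxWalls and eight BP_BoxCorners actors on BeginPlay.
; It needs an existing BP_BoxWalls in the level, reading its WallDims (scaled by 100) for side length and thickness.
; It stores BoxHalfDims and BoxCenter, then spawns each piece offset from the first BP_BoxAssembler found, not from itself.
; One bottom corner lacks the thickness Z offset the other three have.
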(event EventBeginPlay
  (bind _returnvalue (Math|Rotator|MakeRotator 0.0 9e+01 0.0))
  (bind _returnvalue_2 (Math|Rotator|MakeRotator -9e+01 0.0 0.0))
  (bind _returnvalue_3 (Actor|GetActorOfClass "/Game/NewBlueprints/BP_BoxWalls.BP_BoxWalls_C"))
  (bind _asbp_box_walls (Utilities|Casting|CastToBP_BoxWalls _returnvalue_3))
  (Variables|Default|SetBoxHalfDims (/ (Math|Vector|MakeVector (.X (Math|Vector|BreakVector (* (Variables|/Game/NewBlueprints/BP_BoxWalls.BP_BoxWalls_C|GetWallDims _asbp_box_walls) 100))) (.X (Math|Vector|BreakVector (* (Variables|/Game/NewBlueprints/BP_BoxWalls.BP_BoxWalls_C|GetWallDims _asbp_box_walls) 100))) (.X (Math|Vector|BreakVector (* (Variables|/Game/NewBlueprints/BP_BoxWalls.BP_BoxWalls_C|GetWallDims _asbp_box_walls) 100)))) 2))
  (bind _outactors (Actor|GetAllActorsOfClass "BP_BoxAssembler_C"))
  (Variables|Default|SetBoxCenter (+ (Math|Vector|MakeVector (/ (.X (Math|Vector|BreakVector (* (Variables|/Game/NewBlueprints/BP_BoxWalls.BP_BoxWalls_C|GetWallDims _asbp_box_walls) 100))) 2) (/ (.X (Math|Vector|BreakVector (* (Variables|/Game/NewBlueprints/BP_BoxWalls.BP_BoxWalls_C|GetWallDims _asbp_box_walls) 100))) 2) (+ (/ (.X (Math|Vector|BreakVector (* (Variables|/Game/NewBlueprints/BP_BoxWalls.BP_BoxWalls_C|GetWallDims _asbp_box_walls) 100))) 2) (.Z (Math|Vector|BreakVector (* (Variables|/Game/NewBlueprints/BP_BoxWalls.BP_BoxWalls_C|GetWallDims _asbp_box_walls) 100))))) (Transformation|GetActorLocation (Utilities|Array|Get(acopy) _outactors))))
  (Game|SpawnActorfromClass "/Game/NewBlueprints/BP_BoxWalls.BP_BoxWalls_C" (Math|Transform|MakeTransform (Transformation|GetActorLocation (Utilities|Array|Get(acopy) _outactors))) "Undefined" "MultiplyWithRoot" 0 0)
  (Game|SpawnActorfromClass "/Game/NewBlueprints/BP_BoxWalls.BP_BoxWalls_C" (Math|Transform|MakeTransform (+ (Transformation|GetActorLocation (Utilities|Array|Get(acopy) _outactors)) (Math|Vector|MakeVector 0.0 0.0 (+ (.X (Math|Vector|BreakVector (* (Variables|/Game/NewBlueprints/BP_BoxWalls.BP_BoxWalls_C|GetWallDims _asbp_box_walls) 100))) (.Z (Math|Vector|BreakVector (* (Variables|/Game/NewBlueprints/BP_BoxWalls.BP_BoxWalls_C|GetWallDims _asbp_box_walls) 100))))))) "Undefined" "MultiplyWithRoot" 0 0)
  (Game|SpawnActorfromClass "/Game/NewBlueprints/BP_BoxWalls.BP_BoxWalls_C" (Math|Transform|MakeTransform (+ (Transformation|GetActorLocation (Utilities|Array|Get(acopy) _outactors)) (Math|Vector|MakeVector 0.0 0.0 (.Z (Math|Vector|BreakVector (* (Variables|/Game/NewBlueprints/BP_BoxWalls.BP_BoxWalls_C|GetWallDims _asbp_box_walls) 100))))) _returnvalue_2) "Undefined" "MultiplyWithRoot" 0 0)
  (Game|SpawnActorfromClass "/Game/NewBlueprints/BP_BoxWalls.BP_BoxWalls_C" (Math|Transform|MakeTransform (+ (Transformation|GetActorLocation (Utilities|Array|Get(acopy) _outactors)) (Math|Vector|MakeVector 0.0 (+ (.X (Math|Vector|BreakVector (* (Variables|/Game/NewBlueprints/BP_BoxWalls.BP_BoxWalls_C|GetWallDims _asbp_box_walls) 100))) (.Z (Math|Vector|BreakVector (* (Variables|/Game/NewBlueprints/BP_BoxWalls.BP_BoxWalls_C|GetWallDims _asbp_box_walls) 100)))) (.Z (Math|Vector|BreakVector (* (Variables|/Game/NewBlueprints/BP_BoxWalls.BP_BoxWalls_C|GetWallDims _asbp_box_walls) 100))))) _returnvalue_2) "Undefined" "MultiplyWithRoot" 0 0)
  (Game|SpawnActorfromClass "/Game/NewBlueprints/BP_BoxWalls.BP_BoxWalls_C" (Math|Transform|MakeTransform (+ (Transformation|GetActorLocation (Utilities|Array|Get(acopy) _outactors)) (Math|Vector|MakeVector 0.0 0.0 (.Z (Math|Vector|BreakVector (* (Variables|/Game/NewBlueprints/BP_BoxWalls.BP_BoxWalls_C|GetWallDims _asbp_box_walls) 100))))) _returnvalue) "Undefined" "MultiplyWithRoot" 0 0)
  (Game|SpawnActorfromClass "/Game/NewBlueprints/BP_BoxWalls.BP_BoxWalls_C" (Math|Transform|MakeTransform (+ (Transformation|GetActorLocation (Utilities|Array|Get(acopy) _outactors)) (Math|Vector|MakeVector (+ (.X (Math|Vector|BreakVector (* (Variables|/Game/NewBlueprints/BP_BoxWalls.BP_BoxWalls_C|GetWallDims _asbp_box_walls) 100))) (.Z (Math|Vector|BreakVector (* (Variables|/Game/NewBlueprints/BP_BoxWalls.BP_BoxWalls_C|GetWallDims _asbp_box_walls) 100)))) 0.0 (.Z (Math|Vector|BreakVector (* (Variables|/Game/NewBlueprints/BP_BoxWalls.BP_BoxWalls_C|GetWallDims _asbp_box_walls) 100))))) _returnvalue) "Undefined" "MultiplyWithRoot" 0 0)
  (Game|SpawnActorfromClass "/Game/NewBlueprints/BP_BoxCorners.BP_BoxCorners_C" (Math|Transform|MakeTransform (+ (Transformation|GetActorLocation (Utilities|Array|Get(acopy) _outactors)) (Math|Vector|MakeVector 0.0 0.0 (.Z (Math|Vector|BreakVector (* (Variables|/Game/NewBlueprints/BP_BoxWalls.BP_BoxWalls_C|GetWallDims _asbp_box_walls) 100)))))) "Undefined" "MultiplyWithRoot" 0 0)
  (Game|SpawnActorfromClass "/Game/NewBlueprints/BP_BoxCorners.BP_BoxCorners_C" (Math|Transform|MakeTransform (+ (Transformation|GetActorLocation (Utilities|Array|Get(acopy) _outactors)) (Math|Vector|MakeVector (.X (Math|Vector|BreakVector (* (Variables|/Game/NewBlueprints/BP_BoxWalls.BP_BoxWalls_C|GetWallDims _asbp_box_walls) 100))) 0.0 (.Z (Math|Vector|BreakVector (* (Variables|/Game/NewBlueprints/BP_BoxWalls.BP_BoxWalls_C|GetWallDims _asbp_box_walls) 100)))))) "Undefined" "MultiplyWithRoot" 0 0)
  (Game|SpawnActorfromClass "/Game/NewBlueprints/BP_BoxCorners.BP_BoxCorners_C" (Math|Transform|MakeTransform (+ (Transformation|GetActorLocation (Utilities|Array|Get(acopy) _outactors)) (Math|Vector|MakeVector 0.0 (.X (Math|Vector|BreakVector (* (Variables|/Game/NewBlueprints/BP_BoxWalls.BP_BoxWalls_C|GetWallDims _asbp_box_walls) 100))) 0.0))) "Undefined" "MultiplyWithRoot" 0 0)
  (Game|SpawnActorfromClass "/Game/NewBlueprints/BP_BoxCorners.BP_BoxCorners_C" (Math|Transform|MakeTransform (+ (Transformation|GetActorLocation (Utilities|Array|Get(acopy) _outactors)) (Math|Vector|MakeVector (.X (Math|Vector|BreakVector (* (Variables|/Game/NewBlueprints/BP_BoxWalls.BP_BoxWalls_C|GetWallDims _asbp_box_walls) 100))) (.X (Math|Vector|BreakVector (* (Variables|/Game/NewBlueprints/BP_BoxWalls.BP_BoxWalls_C|GetWallDims _asbp_box_walls) 100))) (.Z (Math|Vector|BreakVector (* (Variables|/Game/NewBlueprints/BP_BoxWalls.BP_BoxWalls_C|GetWallDims _asbp_box_walls) 100)))))) "Undefined" "MultiplyWithRoot" 0 0)
  (Game|SpawnActorfromClass "/Game/NewBlueprints/BP_BoxCorners.BP_BoxCorners_C" (Math|Transform|MakeTransform (+ (Transformation|GetActorLocation (Utilities|Array|Get(acopy) _outactors)) (Math|Vector|MakeVector 0.0 0.0 (+ (.X (Math|Vector|BreakVector (* (Variables|/Game/NewBlueprints/BP_BoxWalls.BP_BoxWalls_C|GetWallDims _asbp_box_walls) 100))) (.Z (Math|Vector|BreakVector (* (Variables|/Game/NewBlueprints/BP_BoxWalls.BP_BoxWalls_C|GetWallDims _asbp_box_walls) 100))))))) "Undefined" "MultiplyWithRoot" 0 0)
  (Game|SpawnActorfromClass "/Game/NewBlueprints/BP_BoxCorners.BP_BoxCorners_C" (Math|Transform|MakeTransform (+ (Transformation|GetActorLocation (Utilities|Array|Get(acopy) _outactors)) (Math|Vector|MakeVector (.X (Math|Vector|BreakVector (* (Variables|/Game/NewBlueprints/BP_BoxWalls.BP_BoxWalls_C|GetWallDims _asbp_box_walls) 100))) 0.0 (+ (.X (Math|Vector|BreakVector (* (Variables|/Game/NewBlueprints/BP_BoxWalls.BP_BoxWalls_C|GetWallDims _asbp_box_walls) 100))) (.Z (Math|Vector|BreakVector (* (Variables|/Game/NewBlueprints/BP_BoxWalls.BP_BoxWalls_C|GetWallDims _asbp_box_walls) 100))))))) "Undefined" "MultiplyWithRoot" 0 0)
  (Game|SpawnActorfromClass "/Game/NewBlueprints/BP_BoxCorners.BP_BoxCorners_C" (Math|Transform|MakeTransform (+ (Transformation|GetActorLocation (Utilities|Array|Get(acopy) _outactors)) (Math|Vector|MakeVector 0.0 (.X (Math|Vector|BreakVector (* (Variables|/Game/NewBlueprints/BP_BoxWalls.BP_BoxWalls_C|GetWallDims _asbp_box_walls) 100))) (+ (.X (Math|Vector|BreakVector (* (Variables|/Game/NewBlueprints/BP_BoxWalls.BP_BoxWalls_C|GetWallDims _asbp_box_walls) 100))) (.Z (Math|Vector|BreakVector (* (Variables|/Game/NewBlueprints/BP_BoxWalls.BP_BoxWalls_C|GetWallDims _asbp_box_walls) 100))))))) "Undefined" "MultiplyWithRoot" 0 0)
  (Game|SpawnActorfromClass "/Game/NewBlueprints/BP_BoxCorners.BP_BoxCorners_C" (Math|Transform|MakeTransform (+ (Transformation|GetActorLocation (Utilities|Array|Get(acopy) _outactors)) (Math|Vector|MakeVector (.X (Math|Vector|BreakVector (* (Variables|/Game/NewBlueprints/BP_BoxWalls.BP_BoxWalls_C|GetWallDims _asbp_box_walls) 100))) (.X (Math|Vector|BreakVector (* (Variables|/Game/NewBlueprints/BP_BoxWalls.BP_BoxWalls_C|GetWallDims _asbp_box_walls) 100))) (+ (.X (Math|Vector|BreakVector (* (Variables|/Game/NewBlueprints/BP_BoxWalls.BP_BoxWalls_C|GetWallDims _asbp_box_walls) 100))) (.Z (Math|Vector|BreakVector (* (Variables|/Game/NewBlueprints/BP_BoxWalls.BP_BoxWalls_C|GetWallDims _asbp_box_walls) 100))))))) "Undefined" "MultiplyWithRoot" 0 0))

(fn ConstructionScript)