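; BP_PyramidAssembler racks a 14-ball square pyramid and a cue ball inside the box, apparently for 3D billiards.
; On BeginPlay, BuildPyramid clears all but the first BP_Balls, which supplies ball size and weight.
; It spawns three randomly colored layers around BP_BoxAssembler's center, spaced by ball diameter.
; A heavier white cue ball is placed by retrying random in-box points until clear of the pyramid.
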(event EventBeginPlay
  (CallFunction|BuildPyramid))

(fn ConstructionScript)

(fn BuildPyramid
  (bind _balllocations (Variables|Default|GetBallLocations))
  (bind _balllocations_2 (Variables|Default|GetBallLocations))
  (bind _colorarray (Variables|Default|GetColorArray))
  (bind _colorarray_2 (Variables|Default|GetColorArray))
  (bind _balllocations_3 (Variables|Default|GetBallLocations))
  (bind _balllocations_4 (Variables|Default|GetBallLocations))
  (bind _output (Utilities|Array|Get(acopy) _colorarray_2))
  (while (< (Utilities|Array|Length _colorarray) 14)
    (Utilities|Array|AddUnique _colorarray (Math|Conversions|ToColor(LinearColor) (Math|Color|MakeColor (Math|Random|RandomFloatinRange 0.0 0.7) (Math|Random|RandomFloatinRange 0.0 0.7) (Math|Random|RandomFloatinRange 0.0 0.7)))))
  (bind _outactors (Actor|GetAllActorsOfClass "/Game/NewBlueprints/BP_Balls.BP_Balls_C"))
  (Utilities|Array|RemoveIndex _outactors)
  (if (> (Utilities|Array|Length _outactors) 0)
    (for _array_element _outactors
      (Actor|DestroyActor _array_element)))
  (bind _returnvalue (Actor|GetActorOfClass "/Game/NewBlueprints/BP_BoxAssembler.BP_BoxAssembler_C"))
  (bind _asbp_box_assembler (Utilities|Casting|CastToBP_BoxAssembler _returnvalue))
  (Variables|Default|SetBox%20Center (Variables|/Game/NewBlueprints/BP_BoxAssembler.BP_BoxAssembler_C|GetBoxCenter _asbp_box_assembler))
  (bind _returnvalue_2 (Actor|GetActorOfClass "/Game/NewBlueprints/BP_Balls.BP_Balls_C"))
  (bind _asbp_balls (Utilities|Casting|CastToBP_Balls _returnvalue_2))
  (Game|SpawnActorfromClass "/Game/NewBlueprints/BP_Balls.BP_Balls_C" (Math|Transform|MakeTransform (+ (Variables|Default|GetBox%20Center) (Math|Vector|MakeVector (* (+ (* (Variables|/Game/NewBlueprints/BP_Balls.BP_Balls_C|GetBallDiam _asbp_balls) 1e+02) 1e+01) -1.0) (* (+ (* (Variables|/Game/NewBlueprints/BP_Balls.BP_Balls_C|GetBallDiam _asbp_balls) 1e+02) 1e+01) -1.0) (* (* (Math|Float|Sqrt 2.0) (* (+ (* (Variables|/Game/NewBlueprints/BP_Balls.BP_Balls_C|GetBallDiam _asbp_balls) 1e+02) 1e+01) 0.5)) -1.0)))) "Undefined" "MultiplyWithRoot" 0 (Math|Conversions|ToLinearColor(Color) _output) 0.3 0)
  (Utilities|Array|RemoveIndex _colorarray_2)
  (Utilities|Array|Add _balllocations_3 (+ (Variables|Default|GetBox%20Center) (Math|Vector|MakeVector (* (+ (* (Variables|/Game/NewBlueprints/BP_Balls.BP_Balls_C|GetBallDiam _asbp_balls) 1e+02) 1e+01) -1.0) (* (+ (* (Variables|/Game/NewBlueprints/BP_Balls.BP_Balls_C|GetBallDiam _asbp_balls) 1e+02) 1e+01) -1.0) (* (* (Math|Float|Sqrt 2.0) (* (+ (* (Variables|/Game/NewBlueprints/BP_Balls.BP_Balls_C|GetBallDiam _asbp_balls) 1e+02) 1e+01) 0.5)) -1.0))))
  (Game|SpawnActorfromClass "/Game/NewBlueprints/BP_Balls.BP_Balls_C" (Math|Transform|MakeTransform (+ (Variables|Default|GetBox%20Center) (Math|Vector|MakeVector (* (+ (* (Variables|/Game/NewBlueprints/BP_Balls.BP_Balls_C|GetBallDiam _asbp_balls) 1e+02) 1e+01) -1.0) 0.0 (* (* (Math|Float|Sqrt 2.0) (* (+ (* (Variables|/Game/NewBlueprints/BP_Balls.BP_Balls_C|GetBallDiam _asbp_balls) 1e+02) 1e+01) 0.5)) -1.0)))) "Undefined" "MultiplyWithRoot" 0 (Math|Conversions|ToLinearColor(Color) _output) 0.3 0)
  (Utilities|Array|RemoveIndex _colorarray_2)
  (Utilities|Array|Add _balllocations_3 (+ (Variables|Default|GetBox%20Center) (Math|Vector|MakeVector (* (+ (* (Variables|/Game/NewBlueprints/BP_Balls.BP_Balls_C|GetBallDiam _asbp_balls) 1e+02) 1e+01) -1.0) 0.0 (* (* (Math|Float|Sqrt 2.0) (* (+ (* (Variables|/Game/NewBlueprints/BP_Balls.BP_Balls_C|GetBallDiam _asbp_balls) 1e+02) 1e+01) 0.5)) -1.0))))
  (Game|SpawnActorfromClass "/Game/NewBlueprints/BP_Balls.BP_Balls_C" (Math|Transform|MakeTransform (+ (Variables|Default|GetBox%20Center) (Math|Vector|MakeVector (* (+ (* (Variables|/Game/NewBlueprints/BP_Balls.BP_Balls_C|GetBallDiam _asbp_balls) 1e+02) 1e+01) -1.0) (+ (* (Variables|/Game/NewBlueprints/BP_Balls.BP_Balls_C|GetBallDiam _asbp_balls) 1e+02) 1e+01) (* (* (Math|Float|Sqrt 2.0) (* (+ (* (Variables|/Game/NewBlueprints/BP_Balls.BP_Balls_C|GetBallDiam _asbp_balls) 1e+02) 1e+01) 0.5)) -1.0)))) "Undefined" "MultiplyWithRoot" 0 (Math|Conversions|ToLinearColor(Color) _output) 0.3 0)
  (Utilities|Array|RemoveIndex _colorarray_2)
  (Utilities|Array|Add _balllocations_3 (+ (Variables|Default|GetBox%20Center) (Math|Vector|MakeVector (* (+ (* (Variables|/Game/NewBlueprints/BP_Balls.BP_Balls_C|GetBallDiam _asbp_balls) 1e+02) 1e+01) -1.0) (+ (* (Variables|/Game/NewBlueprints/BP_Balls.BP_Balls_C|GetBallDiam _asbp_balls) 1e+02) 1e+01) (* (* (Math|Float|Sqrt 2.0) (* (+ (* (Variables|/Game/NewBlueprints/BP_Balls.BP_Balls_C|GetBallDiam _asbp_balls) 1e+02) 1e+01) 0.5)) -1.0))))
  (Game|SpawnActorfromClass "/Game/NewBlueprints/BP_Balls.BP_Balls_C" (Math|Transform|MakeTransform (+ (Variables|Default|GetBox%20Center) (Math|Vector|MakeVector 0.0 (* (+ (* (Variables|/Game/NewBlueprints/BP_Balls.BP_Balls_C|GetBallDiam _asbp_balls) 1e+02) 1e+01) -1.0) (* (* (Math|Float|Sqrt 2.0) (* (+ (* (Variables|/Game/NewBlueprints/BP_Balls.BP_Balls_C|GetBallDiam _asbp_balls) 1e+02) 1e+01) 0.5)) -1.0)))) "Undefined" "MultiplyWithRoot" 0 (Math|Conversions|ToLinearColor(Color) _output) 0.3 0)
  (Utilities|Array|RemoveIndex _colorarray_2)
  (Utilities|Array|Add _balllocations_3 (+ (Variables|Default|GetBox%20Center) (Math|Vector|MakeVector 0.0 (* (+ (* (Variables|/Game/NewBlueprints/BP_Balls.BP_Balls_C|GetBallDiam _asbp_balls) 1e+02) 1e+01) -1.0) (* (* (Math|Float|Sqrt 2.0) (* (+ (* (Variables|/Game/NewBlueprints/BP_Balls.BP_Balls_C|GetBallDiam _asbp_balls) 1e+02) 1e+01) 0.5)) -1.0))))
  (Game|SpawnActorfromClass "/Game/NewBlueprints/BP_Balls.BP_Balls_C" (Math|Transform|MakeTransform (+ (Variables|Default|GetBox%20Center) (Math|Vector|MakeVector 0.0 0.0 (* (* (Math|Float|Sqrt 2.0) (* (+ (* (Variables|/Game/NewBlueprints/BP_Balls.BP_Balls_C|GetBallDiam _asbp_balls) 1e+02) 1e+01) 0.5)) -1.0)))) "Undefined" "MultiplyWithRoot" 0 (Math|Conversions|ToLinearColor(Color) _output) 0.3 0)
  (Utilities|Array|RemoveIndex _colorarray_2)
  (Utilities|Array|Add _balllocations_4 (+ (Variables|Default|GetBox%20Center) (Math|Vector|MakeVector 0.0 0.0 (* (* (Math|Float|Sqrt 2.0) (* (+ (* (Variables|/Game/NewBlueprints/BP_Balls.BP_Balls_C|GetBallDiam _asbp_balls) 1e+02) 1e+01) 0.5)) -1.0))))
  (Game|SpawnActorfromClass "/Game/NewBlueprints/BP_Balls.BP_Balls_C" (Math|Transform|MakeTransform (+ (Variables|Default|GetBox%20Center) (Math|Vector|MakeVector 0.0 (+ (* (Variables|/Game/NewBlueprints/BP_Balls.BP_Balls_C|GetBallDiam _asbp_balls) 1e+02) 1e+01) (* (* (Math|Float|Sqrt 2.0) (* (+ (* (Variables|/Game/NewBlueprints/BP_Balls.BP_Balls_C|GetBallDiam _asbp_balls) 1e+02) 1e+01) 0.5)) -1.0)))) "Undefined" "MultiplyWithRoot" 0 (Math|Conversions|ToLinearColor(Color) _output) 0.3 0)
  (Utilities|Array|RemoveIndex _colorarray_2)
  (Utilities|Array|Add _balllocations_4 (+ (Variables|Default|GetBox%20Center) (Math|Vector|MakeVector 0.0 (+ (* (Variables|/Game/NewBlueprints/BP_Balls.BP_Balls_C|GetBallDiam _asbp_balls) 1e+02) 1e+01) (* (* (Math|Float|Sqrt 2.0) (* (+ (* (Variables|/Game/NewBlueprints/BP_Balls.BP_Balls_C|GetBallDiam _asbp_balls) 1e+02) 1e+01) 0.5)) -1.0))))
  (Game|SpawnActorfromClass "/Game/NewBlueprints/BP_Balls.BP_Balls_C" (Math|Transform|MakeTransform (+ (Variables|Default|GetBox%20Center) (Math|Vector|MakeVector (+ (* (Variables|/Game/NewBlueprints/BP_Balls.BP_Balls_C|GetBallDiam _asbp_balls) 1e+02) 1e+01) (* (+ (* (Variables|/Game/NewBlueprints/BP_Balls.BP_Balls_C|GetBallDiam _asbp_balls) 1e+02) 1e+01) -1.0) (* (* (Math|Float|Sqrt 2.0) (* (+ (* (Variables|/Game/NewBlueprints/BP_Balls.BP_Balls_C|GetBallDiam _asbp_balls) 1e+02) 1e+01) 0.5)) -1.0)))) "Undefined" "MultiplyWithRoot" 0 (Math|Conversions|ToLinearColor(Color) _output) 0.3 0)
  (Utilities|Array|RemoveIndex _colorarray_2)
  (Utilities|Array|Add _balllocations_4 (+ (Variables|Default|GetBox%20Center) (Math|Vector|MakeVector (+ (* (Variables|/Game/NewBlueprints/BP_Balls.BP_Balls_C|GetBallDiam _asbp_balls) 1e+02) 1e+01) (* (+ (* (Variables|/Game/NewBlueprints/BP_Balls.BP_Balls_C|GetBallDiam _asbp_balls) 1e+02) 1e+01) -1.0) (* (* (Math|Float|Sqrt 2.0) (* (+ (* (Variables|/Game/NewBlueprints/BP_Balls.BP_Balls_C|GetBallDiam _asbp_balls) 1e+02) 1e+01) 0.5)) -1.0))))
  (Game|SpawnActorfromClass "/Game/NewBlueprints/BP_Balls.BP_Balls_C" (Math|Transform|MakeTransform (+ (Variables|Default|GetBox%20Center) (Math|Vector|MakeVector (+ (* (Variables|/Game/NewBlueprints/BP_Balls.BP_Balls_C|GetBallDiam _asbp_balls) 1e+02) 1e+01) 0.0 (* (* (Math|Float|Sqrt 2.0) (* (+ (* (Variables|/Game/NewBlueprints/BP_Balls.BP_Balls_C|GetBallDiam _asbp_balls) 1e+02) 1e+01) 0.5)) -1.0)))) "Undefined" "MultiplyWithRoot" 0 (Math|Conversions|ToLinearColor(Color) _output) 0.3 0)
  (Utilities|Array|RemoveIndex _colorarray_2)
  (Utilities|Array|Add _balllocations_4 (+ (Variables|Default|GetBox%20Center) (Math|Vector|MakeVector (+ (* (Variables|/Game/NewBlueprints/BP_Balls.BP_Balls_C|GetBallDiam _asbp_balls) 1e+02) 1e+01) 0.0 (* (* (Math|Float|Sqrt 2.0) (* (+ (* (Variables|/Game/NewBlueprints/BP_Balls.BP_Balls_C|GetBallDiam _asbp_balls) 1e+02) 1e+01) 0.5)) -1.0))))
  (Game|SpawnActorfromClass "/Game/NewBlueprints/BP_Balls.BP_Balls_C" (Math|Transform|MakeTransform (+ (Variables|Default|GetBox%20Center) (Math|Vector|MakeVector (+ (* (Variables|/Game/NewBlueprints/BP_Balls.BP_Balls_C|GetBallDiam _asbp_balls) 1e+02) 1e+01) (+ (* (Variables|/Game/NewBlueprints/BP_Balls.BP_Balls_C|GetBallDiam _asbp_balls) 1e+02) 1e+01) (* (* (Math|Float|Sqrt 2.0) (* (+ (* (Variables|/Game/NewBlueprints/BP_Balls.BP_Balls_C|GetBallDiam _asbp_balls) 1e+02) 1e+01) 0.5)) -1.0)))) "Undefined" "MultiplyWithRoot" 0 (Math|Conversions|ToLinearColor(Color) _output) 0.3 0)
  (Utilities|Array|RemoveIndex _colorarray_2)
  (Utilities|Array|Add _balllocations_4 (+ (Variables|Default|GetBox%20Center) (Math|Vector|MakeVector (+ (* (Variables|/Game/NewBlueprints/BP_Balls.BP_Balls_C|GetBallDiam _asbp_balls) 1e+02) 1e+01) (+ (* (Variables|/Game/NewBlueprints/BP_Balls.BP_Balls_C|GetBallDiam _asbp_balls) 1e+02) 1e+01) (* (* (Math|Float|Sqrt 2.0) (* (+ (* (Variables|/Game/NewBlueprints/BP_Balls.BP_Balls_C|GetBallDiam _asbp_balls) 1e+02) 1e+01) 0.5)) -1.0))))
  (Game|SpawnActorfromClass "/Game/NewBlueprints/BP_Balls.BP_Balls_C" (Math|Transform|MakeTransform (+ (Variables|Default|GetBox%20Center) (Math|Vector|MakeVector (* (+ (* (Variables|/Game/NewBlueprints/BP_Balls.BP_Balls_C|GetBallDiam _asbp_balls) 1e+02) 1e+01) 0.5) (* (+ (* (Variables|/Game/NewBlueprints/BP_Balls.BP_Balls_C|GetBallDiam _asbp_balls) 1e+02) 1e+01) 0.5) 0.0))) "Undefined" "MultiplyWithRoot" 0 (Math|Conversions|ToLinearColor(Color) _output) 0.3 0)
  (Utilities|Array|RemoveIndex _colorarray_2)
  (Utilities|Array|Add _balllocations (+ (Variables|Default|GetBox%20Center) (Math|Vector|MakeVector (* (+ (* (Variables|/Game/NewBlueprints/BP_Balls.BP_Balls_C|GetBallDiam _asbp_balls) 1e+02) 1e+01) 0.5) (* (+ (* (Variables|/Game/NewBlueprints/BP_Balls.BP_Balls_C|GetBallDiam _asbp_balls) 1e+02) 1e+01) 0.5) 0.0)))
  (Game|SpawnActorfromClass "/Game/NewBlueprints/BP_Balls.BP_Balls_C" (Math|Transform|MakeTransform (+ (Variables|Default|GetBox%20Center) (Math|Vector|MakeVector (* (+ (* (Variables|/Game/NewBlueprints/BP_Balls.BP_Balls_C|GetBallDiam _asbp_balls) 1e+02) 1e+01) 0.5) (* (+ (* (Variables|/Game/NewBlueprints/BP_Balls.BP_Balls_C|GetBallDiam _asbp_balls) 1e+02) 1e+01) -0.5) 0.0))) "Undefined" "MultiplyWithRoot" 0 (Math|Conversions|ToLinearColor(Color) _output) 0.3 0)
  (Utilities|Array|RemoveIndex _colorarray_2)
  (Utilities|Array|Add _balllocations (+ (Variables|Default|GetBox%20Center) (Math|Vector|MakeVector (* (+ (* (Variables|/Game/NewBlueprints/BP_Balls.BP_Balls_C|GetBallDiam _asbp_balls) 1e+02) 1e+01) 0.5) (* (+ (* (Variables|/Game/NewBlueprints/BP_Balls.BP_Balls_C|GetBallDiam _asbp_balls) 1e+02) 1e+01) -0.5) 0.0)))
  (Game|SpawnActorfromClass "/Game/NewBlueprints/BP_Balls.BP_Balls_C" (Math|Transform|MakeTransform (+ (Variables|Default|GetBox%20Center) (Math|Vector|MakeVector (* (+ (* (Variables|/Game/NewBlueprints/BP_Balls.BP_Balls_C|GetBallDiam _asbp_balls) 1e+02) 1e+01) -0.5) (* (+ (* (Variables|/Game/NewBlueprints/BP_Balls.BP_Balls_C|GetBallDiam _asbp_balls) 1e+02) 1e+01) 0.5) 0.0))) "Undefined" "MultiplyWithRoot" 0 (Math|Conversions|ToLinearColor(Color) _output) 0.3 0)
  (Utilities|Array|RemoveIndex _colorarray_2)
  (Utilities|Array|Add _balllocations (+ (Variables|Default|GetBox%20Center) (Math|Vector|MakeVector (* (+ (* (Variables|/Game/NewBlueprints/BP_Balls.BP_Balls_C|GetBallDiam _asbp_balls) 1e+02) 1e+01) -0.5) (* (+ (* (Variables|/Game/NewBlueprints/BP_Balls.BP_Balls_C|GetBallDiam _asbp_balls) 1e+02) 1e+01) 0.5) 0.0)))
  (Game|SpawnActorfromClass "/Game/NewBlueprints/BP_Balls.BP_Balls_C" (Math|Transform|MakeTransform (+ (Variables|Default|GetBox%20Center) (Math|Vector|MakeVector (* (+ (* (Variables|/Game/NewBlueprints/BP_Balls.BP_Balls_C|GetBallDiam _asbp_balls) 1e+02) 1e+01) -0.5) (* (+ (* (Variables|/Game/NewBlueprints/BP_Balls.BP_Balls_C|GetBallDiam _asbp_balls) 1e+02) 1e+01) -0.5) 0.0))) "Undefined" "MultiplyWithRoot" 0 (Math|Conversions|ToLinearColor(Color) _output) 0.3 0)
  (Utilities|Array|RemoveIndex _colorarray_2)
  (Utilities|Array|Add _balllocations (+ (Variables|Default|GetBox%20Center) (Math|Vector|MakeVector (* (+ (* (Variables|/Game/NewBlueprints/BP_Balls.BP_Balls_C|GetBallDiam _asbp_balls) 1e+02) 1e+01) -0.5) (* (+ (* (Variables|/Game/NewBlueprints/BP_Balls.BP_Balls_C|GetBallDiam _asbp_balls) 1e+02) 1e+01) -0.5) 0.0)))
  (Game|SpawnActorfromClass "/Game/NewBlueprints/BP_Balls.BP_Balls_C" (Math|Transform|MakeTransform (+ (Variables|Default|GetBox%20Center) (Math|Vector|MakeVector 0.0 0.0 (* (Math|Float|Sqrt 2.0) (* (+ (* (Variables|/Game/NewBlueprints/BP_Balls.BP_Balls_C|GetBallDiam _asbp_balls) 1e+02) 1e+01) 0.5))))) "Undefined" "MultiplyWithRoot" 0 (Math|Conversions|ToLinearColor(Color) _output) 0.3 0)
  (Utilities|Array|RemoveIndex _colorarray_2)
  (Utilities|Array|Add _balllocations_2 (+ (Variables|Default|GetBox%20Center) (Math|Vector|MakeVector 0.0 0.0 (* (Math|Float|Sqrt 2.0) (* (+ (* (Variables|/Game/NewBlueprints/BP_Balls.BP_Balls_C|GetBallDiam _asbp_balls) 1e+02) 1e+01) 0.5)))))
  (bind _output_get (Variables|Default|SetBadLocation true))
  (while _output_get
    (Variables|Default|SetBadLocation false)
    (Variables|Default|SetCueBallLocation (Math|Random|RandomPointinBoundingBox (Variables|Default|GetBox%20Center) (- (Variables|/Game/NewBlueprints/BP_BoxAssembler.BP_BoxAssembler_C|GetBoxHalfDims _asbp_box_assembler) (+ (/ (* (Variables|/Game/NewBlueprints/BP_Balls.BP_Balls_C|GetBallDiam _asbp_balls) 1e+02) 2.0) 15.0))))
    (bind _array_element_2 (Utilities|Array|ForEachLoopwithBreak _balllocations_2 :!label _label)
      (:LoopBody
        (if (not (> (Math|Vector|VectorLength (- (Variables|Default|GetCueBallLocation) _array_element_2)) (+ (* (Variables|/Game/NewBlueprints/BP_Balls.BP_Balls_C|GetBallDiam _asbp_balls) 1e+02) 15.0)))
          (Variables|Default|SetBadLocation true)
          (goto _label Break)))))
  (Game|SpawnActorfromClass "/Game/NewBlueprints/BP_Balls.BP_Balls_C" (Math|Transform|MakeTransform (Variables|Default|GetCueBallLocation)) "Undefined" "MultiplyWithRoot" 0 (Math|Color|MakeColor 1.0 1.0 1.0) (* (Variables|/Game/NewBlueprints/BP_Balls.BP_Balls_C|GetBallWeight _asbp_balls) 1.2) 0))