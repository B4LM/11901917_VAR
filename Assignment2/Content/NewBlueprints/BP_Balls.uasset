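; BP_Balls is a ball actor that configures the weight, size and color of its Balls component on BeginPlay.
; It applies BallWeight as mass scale, BallDiam as uniform world scale and BallColorSetter as the BallColor parameter on a dynamic instance of M_Balls.
; It also fills ColorArray with 14 unique random colors, though this graph does not use them for the material.
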(event EventBeginPlay
  (bind _balls (Variables|Default|GetBalls))
  (bind _balldiam (Variables|Default|GetBallDiam))
  (bind _colorarray (Variables|Default|GetColorArray))
  (Class|PrimitiveComponent|SetMassScale (Variables|Default|GetBalls) "None" (Variables|Default|GetBallWeight))
  (while (< (Utilities|Array|Length _colorarray) 14)
    (Utilities|Array|AddUnique _colorarray (Math|Conversions|ToColor(LinearColor) (Math|Color|MakeColor (Math|Random|RandomFloat) (Math|Random|RandomFloat) (Math|Random|RandomFloat)))))
  (bind _returnvalue (Rendering|Material|CreateDynamicMaterialInstance "/Game/NewMaterials/M_Balls.M_Balls" "None" "None" :!class /Script/Engine.KismetMaterialLibrary))
  (Rendering|Material|SetMaterial _balls 0 _returnvalue)
  (Transformation|SetWorldScale3D _balls (Math|Vector|MakeVector _balldiam _balldiam _balldiam))
  (Rendering|Material|SetVectorParameterValue _returnvalue "BallColor" (Variables|Default|GetBallColorSetter) :!class /Script/Engine.MaterialInstanceDynamic))

(fn ConstructionScript)