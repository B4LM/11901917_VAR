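; BP_Queue is a grabbable VR cue, apparently a pool cue, that the player aims with two hands.
; CueAimLeft and CueAimRight start aiming when the opposite hand holds BackHand and VRPawn flags that side as aiming.
; Tick then rotates the actor from BackHand toward the aiming hand until that side's shoot-release input.
; Earlier timer, dispatcher-binding and rotation logic remains disconnected, and debug prints remain.
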(event OnGrabbed(BackHand))

(event OnDropped(BackHand))

(event Custom|UpdateRotation)

(event Custom|AimLeftPressed
  (params (ControllerPosLeft :type Vector)))

(event Custom|AimRightPressed
  (params (ControllerPosRight :type Vector)))

(event Custom|CueAimLeft
  (Development|PrintString "Hello" true true "(R=0.000000,G=0.660000,B=1.000000,A=1.000000)" 1e+03)
  (Variables|Default|SetAimingLeft true)
  (if (Utilities|Enum|Equal(Enum) (Default|GetHeldbyHand (Variables|Default|GetBackHand)) "Right")
    (Development|PrintString "revevrev")
    (bind _returnvalue (Actor|GetActorOfClass "/Game/VRTemplate/Blueprints/VRPawn.VRPawn_C"))
    (bind _asvrpawn (Utilities|Casting|CastToVRPawn _returnvalue))
    (if (Variables|/Game/VRTemplate/Blueprints/VRPawn.VRPawn_C|GetAiming_Left _asvrpawn)
      (Variables|Default|SetStartAimingLeft true)
      (Development|PrintString "StartAiming" true true "(R=1.000000,G=0.045629,B=0.723244,A=1.000000)" 1e+02))))

(event Custom|CueAimRight
  (Development|PrintString "jhguh" true true "(R=0.000000,G=0.660000,B=1.000000,A=1.000000)" 1e+03)
  (Variables|Default|SetAimingRight true)
  (if (Utilities|Enum|Equal(Enum) (Default|GetHeldbyHand (Variables|Default|GetBackHand)) "Left")
    (bind _returnvalue (Actor|GetActorOfClass "/Game/VRTemplate/Blueprints/VRPawn.VRPawn_C"))
    (bind _asvrpawn (Utilities|Casting|CastToVRPawn _returnvalue))
    (if (Variables|/Game/VRTemplate/Blueprints/VRPawn.VRPawn_C|GetAiming_Right _asvrpawn)
      (Variables|Default|SetStartAimingRight true)
      (Development|PrintString "StartAiming" true true "(R=1.000000,G=0.045629,B=0.723244,A=1.000000)" 1e+02))))

(event Input|EnhancedActionEvents|EnhancedInputActionIA_ShootRelease_Left
  (params (ActionValue :type Boolean) (ElapsedSeconds :type Float%20%28double-precision%29) (TriggeredSeconds :type Float%20%28double-precision%29) (InputAction :type Input%20Action%20Object%20Reference :default "/Game/VRTemplate/Input/Actions/IA_ShootRelease_Left.IA_ShootRelease_Left"))
  (Variables|Default|SetAimingLeft false)
  (Variables|Default|SetStartAimingLeft false))

(event Input|EnhancedActionEvents|EnhancedInputActionIA_Shoot_Left
  (params (ActionValue :type Boolean) (ElapsedSeconds :type Float%20%28double-precision%29) (TriggeredSeconds :type Float%20%28double-precision%29) (InputAction :type Input%20Action%20Object%20Reference :default "/Game/VRTemplate/Input/Actions/IA_Shoot_Left.IA_Shoot_Left")))

(event Input|EnhancedActionEvents|EnhancedInputActionIA_Shoot_Right
  (params (ActionValue :type Boolean) (ElapsedSeconds :type Float%20%28double-precision%29) (TriggeredSeconds :type Float%20%28double-precision%29) (InputAction :type Input%20Action%20Object%20Reference :default "/Game/VRTemplate/Input/Actions/IA_Shoot_Right.IA_Shoot_Right")))

(event Input|EnhancedActionEvents|EnhancedInputActionIA_ShootRelease_Right
  (params (ActionValue :type Boolean) (ElapsedSeconds :type Float%20%28double-precision%29) (TriggeredSeconds :type Float%20%28double-precision%29) (InputAction :type Input%20Action%20Object%20Reference :default "/Game/VRTemplate/Input/Actions/IA_ShootRelease_Right.IA_ShootRelease_Right"))
  (Variables|Default|SetAimingRight false)
  (Variables|Default|SetStartAimingRight false))

(event EventBeginPlay)

(event EventTick
  (params (DeltaSeconds :type Float%20%28single-precision%29))
  (if (Variables|Default|GetStartAimingLeft)
    (bind _returnvalue (Actor|GetActorOfClass "/Game/VRTemplate/Blueprints/VRPawn.VRPawn_C"))
    (bind _asvrpawn (Utilities|Casting|CastToVRPawn _returnvalue))
    (Transformation|SetActorRotation (Math|Rotator|FindLookatRotation (Transformation|GetWorldLocation (Variables|Default|GetBackHand)) (Transformation|GetWorldLocation (Variables|/Game/VRTemplate/Blueprints/VRPawn.VRPawn_C|GetHandLeft _asvrpawn))))
    (elif (Variables|Default|GetStartAimingRight)
      (bind _returnvalue_2 (Actor|GetActorOfClass "/Game/VRTemplate/Blueprints/VRPawn.VRPawn_C"))
      (bind _asvrpawn_2 (Utilities|Casting|CastToVRPawn _returnvalue_2))
      (Transformation|SetActorRotation (Math|Rotator|FindLookatRotation (Transformation|GetWorldLocation (Variables|Default|GetBackHand)) (Transformation|GetWorldLocation (Variables|/Game/VRTemplate/Blueprints/VRPawn.VRPawn_C|GetHandRight _asvrpawn_2)))))))

(fn ConstructionScript)